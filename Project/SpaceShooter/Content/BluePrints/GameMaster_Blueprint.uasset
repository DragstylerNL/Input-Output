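; Game master that runs three timed, scripted waves of enemies, then shows a win widget and returns to the main menu.
; Tick accumulates GameTimer to pick the active stage window, using a Delay to throttle stage calls to about one per second.
; Each stage increments StageTime, reset between windows, to trigger hardcoded patterns of single, multiple or full-wall spawns across five evenly spaced lanes.
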(event `self.ReceiveTick`
  (params (DeltaSeconds :type "Float (single-precision)"))
  (bind (_stage_1_x _stage_1_y) (`KismetMathLibrary.BreakVector` (`self.Stage 1`)))
  (bind _gametimer (`self.GameTimer`))
  (bind _gametimer_2 (`self.GameTimer`))
  (bind (_stage_2_x _stage_2_y) (`KismetMathLibrary.BreakVector` (`self.Stage 2`)))
  (bind _gametimer_3 (`self.GameTimer`))
  (bind (_stage_3_x _stage_3_y) (`KismetMathLibrary.BreakVector` (`self.Stage 3`)))
  (set `self.GameTimer` (+ (`self.GameTimer`) DeltaSeconds))
  ;[1 0 0] Stage 1
  (if (> _gametimer _stage_1_x)
    (if (< _gametimer _stage_1_y)
      (`KismetSystemLibrary.Delay` 1.0)
      (`self.Stage1`)
      (else
        ;[1 0 0] Stage 2
        (if (> _gametimer_3 _stage_2_x) :!label _label
          (if (< _gametimer_3 _stage_2_y)
            (`KismetSystemLibrary.Delay` 1.0)
            (`self.Stage2`)
            (else
              ;[1 0 0] Stage 2
              (if (> _gametimer_2 _stage_3_x) :!label _label_2
                (if (< _gametimer_2 _stage_3_y)
                  (`KismetSystemLibrary.Delay` 1.0)
                  (`self.Stage3`)
                  (else
                    ;[1 0 0] End
                    (set `self.StageTime` 0 :!label _label_3)
                    (if (> _gametimer_2 90.0)
                      (bind _returnvalue (`|CreateWidget` "/Game/Win.Win_C"))
                      (`UserWidget.AddToViewport` _returnvalue 0)
                      (`KismetSystemLibrary.Delay` 5.0)
                      (`GameplayStatics.OpenLevel` "MainMenu"))))
                (else
                  (goto _label_3)))))
          (else
            (goto _label_2)))))
    (else
      (goto _label))))

(fn `GetPos`
  (params (posid :type Integer))
  (returns (WorldPosition :type "Vector Structure"))
  (return (+ (`KismetMathLibrary.MakeVector` (`KismetMathLibrary.Conv_IntToDouble` (* posid 110)) 540.0 40.0) 0.0)))

(fn `Spawn`
  (params (Pos :type "Vector Structure"))
  (`|SpawnActorFromClass` "/Game/Enteties/Enemy.Enemy_C" (`KismetMathLibrary.Conv_VectorToTransform` Pos) "Undefined" "OverrideRootScale" null null))

(fn `SpawnMultiple`
  (params (Pos1 :type Integer) (Pos2 :type Integer))
  (`self.SpawnSingle` Pos1)
  (`self.SpawnSingle` Pos2))

(fn `SpawnSingle`
  (params (Pos :type Integer))
  (bind _worldposition (`self.GetPos` Pos))
  (`self.Spawn` _worldposition))

(fn `SpawnWall`
  (`self.SpawnSingle` 2)
  (`self.SpawnSingle` 1)
  (`self.SpawnSingle` 0)
  (`self.SpawnSingle` -1)
  (`self.SpawnSingle` -2))

(fn `Stage1`
  (bind _result (`/Engine/EditorBlueprintResources/StandardMacros.IncrementInt` (`self.StageTime`))
    (:`  `
      (bind _output_get (set `self.StageTime` _result))
      (if (== _output_get 1)
        (`self.SpawnSingle` 0)
        (elif (== _output_get 3)
          (`self.SpawnSingle` 1)
          (elif (== _output_get 5)
            (`self.SpawnSingle` -1)
            (elif (== _output_get 7)
              (`self.SpawnMultiple` 2 -2)
              (elif (== _output_get 9)
                (`self.SpawnMultiple` 2 -2)
                (elif (== _output_get 11)
                  (`self.SpawnSingle` 0)
                  (elif (== _output_get 13)
                    (`self.SpawnSingle` 0)
                    (elif (== _output_get 15)
                      (`self.SpawnMultiple` 1 -1)
                      (elif (== _output_get 17)
                        (`self.SpawnMultiple` 2 -2)
                        (elif (== _output_get 19)
                          (`self.SpawnMultiple` 1 -1))))))))))))))

(fn `Stage2`
  (bind _result (`/Engine/EditorBlueprintResources/StandardMacros.IncrementInt` (`self.StageTime`))
    (:`  `
      (bind _output_get (set `self.StageTime` _result))
      (if (== _output_get 1)
        (`self.SpawnMultiple` 1 -1)
        (elif (== _output_get 3)
          (`self.SpawnMultiple` 1 -1)
          (elif (== _output_get 5)
            (`self.SpawnMultiple` 1 -1)
            (elif (== _output_get 7)
              (`self.SpawnSingle` 0)
              (elif (== _output_get 9)
                (`self.SpawnMultiple` 1 -1)
                (`self.SpawnSingle` 0)
                (elif (== _output_get 11)
                  (`self.SpawnMultiple` 2 -2)
                  (`self.SpawnSingle` 1)
                  (elif (== _output_get 13)
                    (`self.SpawnMultiple` 1 -1)
                    (`self.SpawnMultiple` 2 -2)
                    (elif (== _output_get 15)
                      (`self.SpawnSingle` 0)
                      (elif (== _output_get 17)
                        (`self.SpawnSingle` 0)
                        (elif (== _output_get 19)
                          (`self.SpawnWall`))))))))))))))

(fn `Stage3`
  (bind _result (`/Engine/EditorBlueprintResources/StandardMacros.IncrementInt` (`self.StageTime`))
    (:`  `
      (bind _output_get (set `self.StageTime` _result))
      (if (== _output_get 1)
        (`self.SpawnSingle` 2)
        (elif (== _output_get 2)
          (`self.SpawnSingle` 1)
          (elif (== _output_get 3)
            (`self.SpawnSingle` 0)
            (elif (== _output_get 4)
              (`self.SpawnSingle` -1)
              (elif (== _output_get 5)
                (`self.SpawnSingle` -2)
                (elif (== _output_get 6)
                  (`self.SpawnWall`)
                  (elif (== _output_get 8)
                    (`self.SpawnMultiple` 1 -1)
                    (elif (== _output_get 9)
                      (`self.SpawnMultiple` 2 -2)
                      (elif (== _output_get 11)
                        (`self.SpawnWall`)
                        (elif (== _output_get 14)
                          (`self.SpawnWall`)
                          (elif (== _output_get 15)
                            (`self.SpawnSingle` 0)
                            (elif (== _output_get 16)
                              (`self.SpawnMultiple` 1 -1)
                              (elif (== _output_get 17)
                                (`self.SpawnMultiple` 2 -2)
                                (elif (== _output_get 19)
                                  (`self.SpawnWall`))))))))))))))))))

(fn `UserConstructionScript`)